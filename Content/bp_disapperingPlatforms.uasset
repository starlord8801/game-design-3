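; Disappearing platform that gives way shortly after the third-person character steps on it.
; A Box overlap by the character turns the Floor yellow, then after a short delay hides it and disables its collision.
; Any actor ending overlap with the Box triggers a separate delayed reset that restores the blue material, visibility and collision.
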(event `self.Box.OnComponentBeginOverlap`
  (params (OverlappedComponent :type "PrimitiveComponent Object Reference") (OtherActor :type "Actor Object Reference") (OtherComp :type "PrimitiveComponent Object Reference") (OtherBodyIndex :type Integer) (bFromSweep :type Boolean) (SweepResult :type "HitResult Structure (by ref)"))
  (cast `/Game/ThirdPerson/Blueprints/BP_ThirdPersonCharacter` OtherActor)
  (`PrimitiveComponent.SetMaterial` (`self.floor`) 0 "/Game/Materials/MI_FlatYellow.MI_FlatYellow")
  (`KismetSystemLibrary.Delay` 0.5)
  (`SceneComponent.SetVisibility` (`self.floor`) false false)
  (`PrimitiveComponent.SetCollisionEnabled` (`self.floor`) "NoCollision"))

(event `self.Box.OnComponentEndOverlap`
  (params (OverlappedComponent :type "PrimitiveComponent Object Reference") (OtherActor :type "Actor Object Reference") (OtherComp :type "PrimitiveComponent Object Reference") (OtherBodyIndex :type Integer))
  (`KismetSystemLibrary.Delay` 0.3)
  (`PrimitiveComponent.SetMaterial` (`self.floor`) 0 "/Game/Materials/MI_FlatBlue.MI_FlatBlue")
  (`SceneComponent.SetVisibility` (`self.floor`) true false)
  (`PrimitiveComponent.SetCollisionEnabled` (`self.floor`) "QueryAndPhysics"))

(fn `UserConstructionScript`)